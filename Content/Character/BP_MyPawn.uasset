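; BP_MyPawn is a player pawn Blueprint that turns movement input axes into movement input.
; The forward/backward and strafe axes call MoveForward and MoveRight, which add movement input along the actor's forward and right vectors.
; The CameraZoom axis calls CameraZoomm, which is an empty stub, as are UpdateMovementSpeed, BeginPlay and the construction script.
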(event `self.ReceiveBeginPlay`)

(event `InputAxis|MoveForward/Backward`
  (params (AxisValue :type "Float (single-precision)"))
  (`self.MoveForward` AxisValue))

(event `InputAxis|StrafeLeft/Right`
  (params (AxisValue :type "Float (single-precision)"))
  (`self.MoveRight` AxisValue))

(event `InputAxis CameraZoom`
  (params (Magnitude :type "Float (double-precision)"))
  (`self.CameraZoomm` Magnitude))

(fn `CameraZoomm`
  (params (AxisValue :type "Float (double-precision)")))

(fn `MoveForward`
  (params (AxisValue :type "Float (double-precision)"))
  (`self.AddMovementInput` (`self.GetActorForwardVector`) AxisValue))

(fn `MoveRight`
  (params (AxisValue :type "Float (double-precision)"))
  (`self.AddMovementInput` (`self.GetActorRightVector`) AxisValue))

(fn `UpdateMovementSpeed`)

(fn `UserConstructionScript`)